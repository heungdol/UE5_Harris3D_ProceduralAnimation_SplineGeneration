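; Harris3D spline Blueprint that places icicle meshes on downward-facing bumps of detected mesh geometry and grows them by percentage.
; Point selection keeps Harris3D BUMP vertices whose normals point mostly down, storing flattened indices across all Harris3D sources.
; Initialization builds the spline, resets each point's up vector and rotation, then adds randomly scaled icicle meshes.
; Growth feeds icicle power, delay and Z axis into the shared GrowUpByInfos routine.
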(event EventBeginPlay
  (|CallParentFunction) ; This node is disabled and will not be called.\nDrag off pins to build functionality.
)

(event Collision|EventActorBeginOverlap
  (params (OtherActor :type Actor%20Object%20Reference))
  (|CallParentFunction OtherActor) ; This node is disabled and will not be called.\nDrag off pins to build functionality.
)

(event EventTick
  (params (DeltaSeconds :type Float%20%28single-precision%29))
  (|CallParentFunction DeltaSeconds) ; This node is disabled and will not be called.\nDrag off pins to build functionality.
)

(event EventInitializeHarris3DSpline
  (bind _spline (Variables|Default|GetSpline))
  (bind _outputsuccess (CallFunction|InitSplinePre))
  (if _outputsuccess
    ;[1 1 1] Make Up Vector -> (0, 0, -1)
    (CallFunction|InitSpline)
    (for _index (range 0 (- (Spline|GetNumberOfSplinePoints (Variables|Default|GetSpline)) 1))
      (Class|SplineComponent|SetUpVectoratSplinePoint _spline _index (Math|Vector|MakeVector 0.0 0.0 1.0) "World" true)
      (Spline|SetRotationatSplinePoint _spline _index (Math|Rotator|MakeRotator 0.0 0.0 0.0) "World" true))
    (CallFunction|InitSplineMeshPoint _spline (Variables|Default|Geticicle_mesh) "X" (Variables|Default|Geticicle_scale) (Variables|Default|Geticicle_scale_random) 0.0)))

(fn ConstructionScript)

(fn GetPointfromHarris3DIcicle
  (params (inputHarris3D :type My%20Harris%203D%20Object%20Reference)))

(fn GetPointsfromHarris3D
  (params (inputStartPoints :type Vector :default "0, 0, 0"))
  (for _index (range 0 (- (Utilities|Array|Length (Variables|Default|GetmyHarris3Ds)) 1))
    (for _index_2 (range 0 (- (Utilities|Array|Length (Variables|/Script/Harris3D.MyHarris3D|GetvrtTypes_postSelected (Utilities|Array|Get(acopy) (Variables|Default|GetmyHarris3Ds) _index))) 1))
      ;[1 1 1] Find Bump Vertex and Insert Index Buffer
      (if (and (Utilities|Enum|Equal(Enum) (Utilities|Array|Get(acopy) (Variables|/Script/Harris3D.MyHarris3D|GetvrtTypes_postSelected (Utilities|Array|Get(acopy) (Variables|Default|GetmyHarris3Ds) _index)) _index_2) (Utilities|Enum|LiteralenumEVertexType "VERTEX_BUMP")) (> (Math|Vector|DotProduct (Utilities|Array|Get(acopy) (Variables|/Script/Harris3D.MyHarris3D|GetcurrentVrtNors_postSelected (Utilities|Array|Get(acopy) (Variables|Default|GetmyHarris3Ds) _index)) _index_2) "0, 0,-1.000000") 0.5))
        (Utilities|Array|Add (Variables|Default|GetindexBufferArray) (+ _index_2 (* _index (Variables|Default|GetvertexNum_max))))))))

(fn GrowUpbyPercentage
  (params (inputPercentage :type Float%20%28double-precision%29))
  (Utilities|Array|Clear (LocalVariables|Getpowers))
  (Utilities|Array|Clear (LocalVariables|Getdelays))
  (Utilities|Array|Clear (LocalVariables|Getaxises))
  (Utilities|Array|Add (LocalVariables|Getpowers) (Variables|Default|Geticicle_growth_power))
  (Utilities|Array|Add (LocalVariables|Getdelays) (Variables|Default|Geticicle_growth_delay))
  (Utilities|Array|Add (LocalVariables|Getaxises) "0.000000,0.000000,1.000000")
  (CallFunction|GrowUpbyInfos inputPercentage 0.0 0.0 (LocalVariables|Getpowers) (LocalVariables|Getdelays) (LocalVariables|Getaxises)))