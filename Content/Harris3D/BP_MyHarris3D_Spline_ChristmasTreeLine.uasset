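; Harris3D spline actor that builds a Christmas tree garland line with light meshes over selected Harris3D vertices.
; Point selection steps up a virtual spiralling cone at the actor's location, taking the nearest vertex within a distance band at each step and stopping at the first miss.
; Initialization applies vertical tangents to the spline, then lays the line as pipe meshes and spaces randomly scaled lights along it.
; GrowUpByPercentage ignores its input and always passes full growth.
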(event EventBeginPlay
  (|CallParentFunction) ; This node is disabled and will not be called.\nDrag off pins to build functionality.
)

(event Collision|EventActorBeginOverlap
  (params (OtherActor :type Actor%20Object%20Reference))
  (|CallParentFunction OtherActor) ; This node is disabled and will not be called.\nDrag off pins to build functionality.
)

(event EventTick
  (params (DeltaSeconds :type Float%20%28single-precision%29))
  (|CallParentFunction DeltaSeconds) ; This node is disabled and will not be called.\nDrag off pins to build functionality.
)

(event EventInitializeHarris3DSpline
  (bind _spline (Variables|Default|GetSpline))
  (bind _outputsuccess (CallFunction|InitSplinePre))
  (if _outputsuccess
    (CallFunction|InitSpline)
    (for _index (range 0 (- (Spline|GetNumberOfSplinePoints (Variables|Default|GetSpline)) 1))
      (Spline|SetTangentsatSplinePoint (Variables|Default|GetSpline) _index (Math|Vector|MakeVector 0.0 0.0 1e+02) (Math|Vector|MakeVector 0.0 0.0 -1e+02) "Local" true))
    (CallFunction|InitSplineMeshPipe _spline (Variables|Default|GettreeLine_mesh) (Variables|Default|GettreeLine_mesh_axis) (Variables|Default|GettreeLine_mesh_scale) 1.0 0.0 (Variables|Default|GettreeLine_offset))
    (CallFunction|InitSplineMeshDistance _spline (Variables|Default|GettreeLineLight_mesh) (Variables|Default|GettreeLineLight_mesh_axis) (Variables|Default|GettreeLineLight_mesh_scale) (Variables|Default|GettreeLineLight_mesh_scale_random) 1.0 0.7 (Variables|Default|GettreeLineLight_mesh_space) (Variables|Default|GettreeLineLight_offset))))

(fn ConstructionScript)

(fn GetPointfromHarris3DTreeLine
  (params (inputHarris3D :type My%20Harris%203D%20Object%20Reference) (inputDistMin :type Float%20%28double-precision%29) (inputDistMax :type Float%20%28double-precision%29) (inputTreeRadius :type Float%20%28double-precision%29) (inputTreeHeight :type Float%20%28double-precision%29) (inputTreePartitionNumber :type Integer) (inputTreePartitionNumber_rotation :type Integer) (inputTreeCount :type Integer))
  (bind _returnvalue (Math|Conversions|ToFloat(Integer) inputTreePartitionNumber_rotation))
  (bind _returnvalue_2 (/ 3.6e+02 _returnvalue))
  (bind _returnvalue_3 (* _returnvalue_2 inputTreeCount))
  (bind _returnvalue_4 (/ _returnvalue_3 1.8e+02))
  (bind _returnvalue_5 (Math|Float|MultiplybyPi _returnvalue_4))
  (if (<= (Utilities|Array|Length (Variables|/Script/Harris3D.MyHarris3D|GetcurrentVrtLocs_postSelected inputHarris3D)) 0)
    (return -1)
    (else
      (LocalVariables|SetcurrentIndex -1)
      (LocalVariables|SetcurrentDist 1e+04)
      (for _index (range 0 (- (Utilities|Array|Length (Variables|/Script/Harris3D.MyHarris3D|GetcurrentVrtLocs_postSelected inputHarris3D)) 1))
        ;[1 1 1] Dist
        (if (and (> (Math|Vector|Distance(Vector) (+ (+ (* (Math|Vector|MakeVector (Math|Trig|Cos(Radians) _returnvalue_5) (Math|Trig|Sin(Radians) _returnvalue_5) 0.0) (* (/ inputTreeRadius (+ inputTreePartitionNumber 1)) (- (+ inputTreePartitionNumber 1) inputTreeCount))) (Math|Vector|MakeVector 0.0 0.0 (* (/ inputTreeHeight (+ inputTreePartitionNumber 1)) inputTreeCount))) (Transformation|GetWorldLocation (Variables|Default|GetDefaultSceneRoot))) (Utilities|Array|Get(acopy) (Variables|/Script/Harris3D.MyHarris3D|GetcurrentVrtLocs_postSelected inputHarris3D) _index)) inputDistMin) (< (Math|Vector|Distance(Vector) (+ (+ (* (Math|Vector|MakeVector (Math|Trig|Cos(Radians) _returnvalue_5) (Math|Trig|Sin(Radians) _returnvalue_5) 0.0) (* (/ inputTreeRadius (+ inputTreePartitionNumber 1)) (- (+ inputTreePartitionNumber 1) inputTreeCount))) (Math|Vector|MakeVector 0.0 0.0 (* (/ inputTreeHeight (+ inputTreePartitionNumber 1)) inputTreeCount))) (Transformation|GetWorldLocation (Variables|Default|GetDefaultSceneRoot))) (Utilities|Array|Get(acopy) (Variables|/Script/Harris3D.MyHarris3D|GetcurrentVrtLocs_postSelected inputHarris3D) _index)) inputDistMax))
          ;[1 1 1] Best
          (if (< (Math|Vector|Distance(Vector) (+ (+ (* (Math|Vector|MakeVector (Math|Trig|Cos(Radians) _returnvalue_5) (Math|Trig|Sin(Radians) _returnvalue_5) 0.0) (* (/ inputTreeRadius (+ inputTreePartitionNumber 1)) (- (+ inputTreePartitionNumber 1) inputTreeCount))) (Math|Vector|MakeVector 0.0 0.0 (* (/ inputTreeHeight (+ inputTreePartitionNumber 1)) inputTreeCount))) (Transformation|GetWorldLocation (Variables|Default|GetDefaultSceneRoot))) (Utilities|Array|Get(acopy) (Variables|/Script/Harris3D.MyHarris3D|GetcurrentVrtLocs_postSelected inputHarris3D) _index)) (LocalVariables|GetcurrentDist))
            (LocalVariables|SetcurrentDist (Math|Vector|Distance(Vector) (+ (+ (* (Math|Vector|MakeVector (Math|Trig|Cos(Radians) _returnvalue_5) (Math|Trig|Sin(Radians) _returnvalue_5) 0.0) (* (/ inputTreeRadius (+ inputTreePartitionNumber 1)) (- (+ inputTreePartitionNumber 1) inputTreeCount))) (Math|Vector|MakeVector 0.0 0.0 (* (/ inputTreeHeight (+ inputTreePartitionNumber 1)) inputTreeCount))) (Transformation|GetWorldLocation (Variables|Default|GetDefaultSceneRoot))) (Utilities|Array|Get(acopy) (Variables|/Script/Harris3D.MyHarris3D|GetcurrentVrtLocs_postSelected inputHarris3D) _index)))
            (LocalVariables|SetcurrentIndex _index))))
      (return (LocalVariables|GetcurrentIndex)))))

(fn GetPointsfromHarris3D
  (params (inputStartPoints :type Vector :default "0, 0, 0"))
  (LocalVariables|SetloopLocation inputStartPoints)
  (LocalVariables|SetloopCondition true)
  (bind _index (Utilities|FlowControl|ForLoopwithBreak 0 (- (Utilities|Array|Length (Variables|Default|GetmyHarris3Ds)) 1) :!label _label)
    (:LoopBody
      (if (LocalVariables|GetloopCondition)
        (bind _index_2 (Utilities|FlowControl|ForLoopwithBreak 0 (+ (Variables|Default|GettreeLine_treePartitionNumber) 1) :!label _label_2)
          (:LoopBody
            (if (LocalVariables|GetloopCondition)
              (bind _outputindex (CallFunction|GetPointfromHarris3DTreeLine (Utilities|Array|Get(acopy) (Variables|Default|GetmyHarris3Ds) _index) (Variables|Default|Getspline_detect_dist_min) (Variables|Default|Getspline_detect_dist_max) (Variables|Default|GettreeLine_treeRadius) (Variables|Default|GettreeLine_treeHeight) (Variables|Default|GettreeLine_treePartitionNumber) (Variables|Default|GettreeLine_treePartitionNumber_circle) _index_2))
              (if (== _outputindex -1)
                (LocalVariables|SetloopCondition false)
                (else
                  (LocalVariables|SetloopLocation (Utilities|Array|Get(acopy) (Variables|/Script/Harris3D.MyHarris3D|GetcurrentVrtLocs_postSelected (Utilities|Array|Get(acopy) (Variables|Default|GetmyHarris3Ds) _index)) _outputindex))
                  (Utilities|Array|Add (Variables|Default|GetindexBufferArray) (+ _outputindex (* _index (Variables|Default|GetvertexNum_max))))))
              (else
                (goto _label_2 Break)))))
        (else
          (goto _label Break))))))

(fn GrowUpbyPercentage
  (params (inputPercentage :type Float%20%28double-precision%29))
  (bind _powers (LocalVariables|Getpowers))
  (bind _delays (LocalVariables|Getdelays))
  (Utilities|Array|Clear _powers)
  (Utilities|Array|Clear _delays)
  (Utilities|Array|Clear (LocalVariables|Getaxises))
  (Utilities|Array|Add _powers 1.0)
  (Utilities|Array|Add _delays 1.0)
  (Utilities|Array|Add (LocalVariables|Getaxises) "1.000000,1.000000,1.000000")
  (CallFunction|GrowUpbyInfos 1.0 1.0 0.0 (LocalVariables|Getpowers) (LocalVariables|Getdelays) (LocalVariables|Getaxises)))