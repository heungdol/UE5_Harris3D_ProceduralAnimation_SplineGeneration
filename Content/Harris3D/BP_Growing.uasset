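; BP_Growing is a Blueprint that animates growth on a set of Harris3DSpline objects over time.
; Every tick it advances GrowthPercentage by delta time over GrowDuration, with no clamp, then calls GrowUp.
; GrowUp passes the stored GrowthPercentage, rather than its input, to GrowUpByPercentage on each spline.
; BeginPlay sets IsGrowing when the spline array is non-empty, but Tick does not check it.
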(event Custom|GrowUp
  (params (inputPercentage :type Float%20%28double-precision%29))
  (for _array_element (Variables|Default|Getharris3DSpline)
    (Default|GrowUpbyPercentage _array_element (Variables|Default|GetgrowthPercentage))))

(event EventBeginPlay
  (Variables|Default|SetisGrowing (> (Utilities|Array|Length (Variables|Default|Getharris3DSpline)) 0)))

(event Collision|EventActorBeginOverlap
  (params (OtherActor :type Actor%20Object%20Reference)))

(event EventTick
  (params (DeltaSeconds :type Float%20%28single-precision%29))
  (Variables|Default|SetgrowthPercentage (+ (Variables|Default|GetgrowthPercentage) (/ DeltaSeconds (Variables|Default|GetgrowDuration))))
  (CallFunction|GrowUp (Variables|Default|GetgrowthPercentage)))

(fn ConstructionScript)