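; Base spline actor that builds growable pipe and prop meshes through points selected by MyHarris3D objects.
; InitSpline refreshes those sources, fills an index buffer through the overridable, empty GetPointsFromHarris3D, then places spline points using vertex normals for up vectors and tangents.
; Helpers add tapered spline meshes or seeded random static meshes by distance or point.
; GrowUpByInfos replays cached scales as staggered growth from a percentage; GrowUpByPercentage is an empty stub.
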(event EventBeginPlay)

(event Collision|EventActorBeginOverlap
  (params (OtherActor :type Actor%20Object%20Reference)))

(event EventTick
  (params (DeltaSeconds :type Float%20%28single-precision%29)))

(event EventInitializeHarris3DSpline
  (bind _outputsuccess (CallFunction|InitSplinePre))
  (if _outputsuccess
    (CallFunction|InitSpline)))

(fn ConstructionScript)

(fn GetPointsfromHarris3D
  (params (inputStartPoints :type Vector)))

(fn InitSplinePre
  ;[1 1 1] Check is Valid
  (if (> (Utilities|Array|Length (Variables|Default|GetmyHarris3Ds)) 0)
    ;[1 1 1] Check Harris 3D First Update
    (for _array_element (Variables|Default|GetmyHarris3Ds)
      (bind _returnvalue (Class|MyHarris3D|GetIsUpdated _array_element))
      (if (not _returnvalue)
        (Class|MyHarris3D|UpdateHarris3D _array_element)))
    (return true)))

(fn InitSpline
  (bind _spline (Variables|Default|GetSpline))
  (bind _spline_2 (Variables|Default|GetSpline))
  (bind _tangentmul_normal (Variables|Default|GettangentMul_normal))
  (bind _spline_3 (Variables|Default|GetSpline))
  (bind _returnvalue (Transformation|GetWorldLocation _spline))
  ;[1 1 1] Clear Array
  (Utilities|Array|Clear (Variables|Default|GetsplineMeshes))
  (Utilities|Array|Clear (Variables|Default|GetsplineMeshes_scale))
  (Utilities|Array|Clear (Variables|Default|GetstaticMeshes))
  (Utilities|Array|Clear (Variables|Default|GetstaticMeshes_scale))
  (Utilities|Array|Clear (Variables|Default|GetstaticMeshes_num))
  ;[1 1 1] Is Valid -> Init_Pre
  (Utilities|Array|Clear (Variables|Default|GetindexBufferArray))
  ;[1 1 1] First Spline Point
  (Spline|ClearSplinePoints _spline_3 true)
  (Spline|AddSplinePoint _spline_3 _returnvalue "World" true)
  ;[1 1 1] Getting Points (Overrided)
  (CallFunction|GetPointsfromHarris3D _returnvalue)
  ;[1 1 1] Making Spline According to Index Array
  (for (_array_element _array_index) (Variables|Default|GetindexBufferArray)
    (Spline|AddSplinePoint _spline_2 (Utilities|Array|Get(acopy) (Variables|/Script/Harris3D.MyHarris3D|GetcurrentVrtLocs_postSelected (Utilities|Array|Get(acopy) (Variables|Default|GetmyHarris3Ds) (/ _array_element (Variables|Default|GetvertexNum_max)))) (Math|Integer|%(Integer) _array_element (Variables|Default|GetvertexNum_max))) "World" true)
    (Class|SplineComponent|SetUpVectoratSplinePoint _spline_2 _array_index (Utilities|Array|Get(acopy) (Variables|/Script/Harris3D.MyHarris3D|GetcurrentVrtNors_postSelected (Utilities|Array|Get(acopy) (Variables|Default|GetmyHarris3Ds) (/ _array_element (Variables|Default|GetvertexNum_max)))) (Math|Integer|%(Integer) _array_element (Variables|Default|GetvertexNum_max))) "World" true)
    (Spline|SetTangentsatSplinePoint _spline_2 _array_index (+ (* (* (Utilities|Array|Get(acopy) (Variables|/Script/Harris3D.MyHarris3D|GetcurrentVrtNors_postSelected (Utilities|Array|Get(acopy) (Variables|Default|GetmyHarris3Ds) (/ _array_element (Variables|Default|GetvertexNum_max)))) (Math|Integer|%(Integer) _array_element (Variables|Default|GetvertexNum_max))) (Math|Vector|MakeVector _tangentmul_normal _tangentmul_normal _tangentmul_normal)) (Math|Vector|MakeVector -1.0 -1.0 -1.0)) (Spline|GetArriveTangentatSplinePoint _spline_2 _array_index "World")) (+ (* (Utilities|Array|Get(acopy) (Variables|/Script/Harris3D.MyHarris3D|GetcurrentVrtNors_postSelected (Utilities|Array|Get(acopy) (Variables|Default|GetmyHarris3Ds) (/ _array_element (Variables|Default|GetvertexNum_max)))) (Math|Integer|%(Integer) _array_element (Variables|Default|GetvertexNum_max))) (Math|Vector|MakeVector _tangentmul_normal _tangentmul_normal _tangentmul_normal)) (Spline|GetLeaveTangentatSplinePoint _spline_2 _array_index "World")) "World" true)))

(fn InitSplineMeshPipe
  (params (inputSpline :type Spline%20Component%20Object%20Reference) (inputSplineMesh :type Static%20Mesh%20Object%20Reference) (inputSplineMeshAxis :type ESplineMeshAxis%20Enum :default "X") (inputScale_total :type Float%20%28double-precision%29) (inputScale_first :type Float%20%28double-precision%29) (inputScale_last :type Float%20%28double-precision%29) (inputOffset :type Float%20%28double-precision%29))
  (bind _splinemeshes (Variables|Default|GetsplineMeshes))
  (bind _returnvalue (Spline|GetNumberOfSplinePoints inputSpline))
  (bind _returnvalue_2 (* inputScale_last inputScale_total))
  (bind _returnvalue_3 (* inputScale_first inputScale_total))
  (bind _returnvalue_4 (+ _returnvalue_2 0.0))
  (bind _returnvalue_5 (+ _returnvalue_3 0.0))
  (bind _returnvalue_6 (- _returnvalue 1))
  (bind _returnvalue_7 (Math|Conversions|ToFloat(Integer) _returnvalue_6))
  ;[1 1 1] Is Valid
  (if (and (Utilities|IsValid inputSpline) (Utilities|IsValid inputSplineMesh))
    ;[1 1 1] Create Spline Mesh
    (for _index (range 0 (- (Spline|GetNumberOfSplinePoints inputSpline) 2))
      (bind _returnvalue_8 (AddComponent|AddSplineMeshComponent false))
      (Components|StaticMesh|SetStaticMesh _returnvalue_8 inputSplineMesh)
      (SplineMesh|SetForwardAxis _returnvalue_8 inputSplineMeshAxis true)
      (SplineMesh|SetStartandEnd _returnvalue_8 (+ (.Location (Spline|GetLocationandTangentatSplinePoint inputSpline _index "World")) (* (Class|SplineComponent|GetUpVectoratSplinePoint inputSpline _index "World") inputOffset)) (.Tangent (Spline|GetLocationandTangentatSplinePoint inputSpline _index "World")) (+ (.Location (Spline|GetLocationandTangentatSplinePoint inputSpline (+ _index 1) "World")) (* (Class|SplineComponent|GetUpVectoratSplinePoint inputSpline (+ _index 1) "World") inputOffset)) (* (.Tangent (Spline|GetLocationandTangentatSplinePoint inputSpline (+ _index 1) "World")) "-1.000000,-1.000000,-1.000000") true :!class /Script/Engine.SplineMeshComponent)
      (SplineMesh|SetStartScale _returnvalue_8 (Math|Vector2D|MakeVector2D (Math|Float|Lerp _returnvalue_5 _returnvalue_4 (/ (- _index 1) _returnvalue_7)) (Math|Float|Lerp _returnvalue_5 _returnvalue_4 (/ (- _index 1) _returnvalue_7))) true :!class /Script/Engine.SplineMeshComponent)
      (SplineMesh|SetEndScale _returnvalue_8 (Math|Vector2D|MakeVector2D (Math|Float|Lerp _returnvalue_5 _returnvalue_4 (/ (Math|Conversions|ToFloat(Integer) _index) _returnvalue_7)) (Math|Float|Lerp _returnvalue_5 _returnvalue_4 (/ (Math|Conversions|ToFloat(Integer) _index) _returnvalue_7))) true :!class /Script/Engine.SplineMeshComponent)
      (SplineMesh|SetSplineUpDir _returnvalue_8 (Class|SplineComponent|GetUpVectoratSplinePoint inputSpline _index "World") true)
      (Utilities|Array|Add (Variables|Default|GetsplineMeshes) _returnvalue_8)
      (Utilities|Array|Add (Variables|Default|GetsplineMeshes_scale) (Math|Vector2D|MakeVector2D (Math|Float|Lerp _returnvalue_5 _returnvalue_4 (/ (- _index 1) _returnvalue_7)) (Math|Float|Lerp _returnvalue_5 _returnvalue_4 (/ (- _index 1) _returnvalue_7)))))
    ;[1 1 1] Post Process for Growth System
    (Utilities|Array|Add (Variables|Default|GetsplineMeshes_scale) (SplineMesh|GetEndScale (Utilities|Array|Get(acopy) _splinemeshes (- (Utilities|Array|Length _splinemeshes) 1))))))

(fn InitSplineMeshDistance
  (params (inputSpline :type Spline%20Component%20Object%20Reference) (inputSplineMesh :type Array%20of%20Static%20Mesh%20Object%20References) (inputSplineMeshAxis :type ESplineMeshAxis%20Enum :default "X") (inputScale :type Vector) (inputScale_random :type Vector) (inputScale_first :type Float%20%28double-precision%29) (inputScale_last :type Float%20%28double-precision%29) (inputScale_space :type Float%20%28double-precision%29) (inputOffset :type Float%20%28double-precision%29))
  ;[1 1 1] Is Valid
  (if (and (Utilities|IsValid inputSpline) (> (Utilities|Array|Length inputSplineMesh) 0))
    ;[1 1 1] Create Static Mesh by Distance
    (LocalVariables|Setcount 0)
    (for _index (range 0 (Math|Float|Truncate (/ (Spline|GetSplineLength inputSpline) inputScale_space)))
      (if (not (== _index 0))
        (bind _returnvalue (AddComponent|AddStaticMeshComponent true (Math|Transform|MakeTransform (+ (Spline|GetLocationatDistanceAlongSpline inputSpline (* (Math|Conversions|ToFloat(Integer) _index) inputScale_space) "World") (* (Class|SplineComponent|GetUpVectoratDistanceAlongSpline inputSpline (* (Math|Conversions|ToFloat(Integer) _index) inputScale_space) "World") inputOffset)) (Spline|GetRotationatDistanceAlongSpline inputSpline (* (Math|Conversions|ToFloat(Integer) _index) inputScale_space) "World"))))
        (Components|StaticMesh|SetStaticMesh _returnvalue (Utilities|Array|Get(acopy) inputSplineMesh (Math|Random|RandomIntegerinRangefromStream 0 (- (Utilities|Array|Length inputSplineMesh) 1) (Variables|Default|GetrandomSeed))))
        (Transformation|SetRelativeScale3D _returnvalue (* (Math|Float|Clamp(Float) (/ (Math|Conversions|ToFloat(Integer) _index) (/ (Spline|GetSplineLength inputSpline) inputScale_space)) inputScale_first inputScale_last) (Math|Vector|Lerp(Vector) inputScale inputScale_random (Math|Random|RandomFloatfromStream (Variables|Default|GetrandomSeed)))))
        (Utilities|Array|Add (Variables|Default|GetstaticMeshes) _returnvalue)
        (Utilities|Array|Add (Variables|Default|GetstaticMeshes_scale) (* (Math|Float|Clamp(Float) (/ (Math|Conversions|ToFloat(Integer) _index) (/ (Spline|GetSplineLength inputSpline) inputScale_space)) inputScale_first inputScale_last) (Math|Vector|Lerp(Vector) inputScale inputScale_random (Math|Random|RandomFloatfromStream (Variables|Default|GetrandomSeed)))))
        (LocalVariables|Setcount (+ (LocalVariables|Getcount) 1))))
    ;[1 1 1] Post Process for Growth System
    (Utilities|Array|Add (Variables|Default|GetstaticMeshes_num) (LocalVariables|Getcount))))

(fn InitSplineMeshPoint
  (params (inputSpline :type Spline%20Component%20Object%20Reference) (inputSplineMesh :type Array%20of%20Static%20Mesh%20Object%20References) (inputSplineMeshAxis :type ESplineMeshAxis%20Enum :default "X") (inputScale :type Vector) (inputScale_random :type Vector) (inputOffset :type Float%20%28double-precision%29))
  (bind _randomseed (Variables|Default|GetrandomSeed))
  (bind _returnvalue (Math|Random|RandomFloatfromStream _randomseed))
  (bind _returnvalue_2 (Math|Vector|Lerp(Vector) inputScale inputScale_random _returnvalue))
  ;[1 1 1] Is Valid
  (if (and (Utilities|IsValid inputSpline) (> (Utilities|Array|Length inputSplineMesh) 0))
    ;[1 1 1] Create Static Mesh by Points
    (LocalVariables|Setcount 0)
    (for _index (range 1 (- (Spline|GetNumberOfSplinePoints inputSpline) 1))
      (bind _returnvalue_3 (AddComponent|AddStaticMeshComponent true (Math|Transform|MakeTransform (+ (Spline|GetLocationatSplinePoint inputSpline _index "World") (* (Class|SplineComponent|GetUpVectoratSplinePoint inputSpline _index "World") inputOffset)) (Spline|GetRotationatSplinePoint inputSpline _index "World"))))
      (Components|StaticMesh|SetStaticMesh _returnvalue_3 (Utilities|Array|Get(acopy) inputSplineMesh (Math|Random|RandomIntegerinRangefromStream 0 (- (Utilities|Array|Length inputSplineMesh) 1) (Variables|Default|GetrandomSeed))))
      (Transformation|SetRelativeScale3D _returnvalue_3 _returnvalue_2)
      (Utilities|Array|Add (Variables|Default|GetstaticMeshes) _returnvalue_3)
      (Utilities|Array|Add (Variables|Default|GetstaticMeshes_scale) _returnvalue_2)
      (LocalVariables|Setcount (+ (LocalVariables|Getcount) 1)))
    ;[1 1 1] Post Process for Growth System
    (Utilities|Array|Add (Variables|Default|GetstaticMeshes_num) (LocalVariables|Getcount))))

(fn GrowUpbyInfos
  (params (inputPercentage :type Float%20%28double-precision%29) (inputPower :type Float%20%28double-precision%29) (inputDelay :type Float%20%28double-precision%29) (inputPower_staticMesh :type Array%20of%20Floats%20%28double-precision%29) (inputDelay_staticMesh :type Array%20of%20Floats%20%28double-precision%29) (inputAxis_staticMesh :type Array%20of%20Vectors))
  (bind _splinemeshes (Variables|Default|GetsplineMeshes))
  (Utilities|FlowControl|Sequence
    (:then_0
      ;[1 1 1] Spline -> OnlyOne
      (for (_array_element _array_index) _splinemeshes
        (SplineMesh|SetStartScale _array_element (* (Utilities|Array|Get(acopy) (Variables|Default|GetsplineMeshes_scale) _array_index) (Math|Vector2D|MakeVector2D (Math|Float|Power (Math|Float|Min(Float) (/ (Math|Float|Max(Float) (- inputPercentage (/ (Math|Conversions|ToFloat(Integer) _array_index) (Math|Conversions|ToFloat(Integer) (Utilities|Array|Length _splinemeshes)))) 0.0) inputDelay) 1.0) inputPower) (Math|Float|Power (Math|Float|Min(Float) (/ (Math|Float|Max(Float) (- inputPercentage (/ (Math|Conversions|ToFloat(Integer) _array_index) (Math|Conversions|ToFloat(Integer) (Utilities|Array|Length _splinemeshes)))) 0.0) inputDelay) 1.0) inputPower))) true :!class /Script/Engine.SplineMeshComponent)
        (SplineMesh|SetEndScale _array_element (* (Utilities|Array|Get(acopy) (Variables|Default|GetsplineMeshes_scale) (+ _array_index 1)) (Math|Vector2D|MakeVector2D (Math|Float|Power (Math|Float|Min(Float) (/ (Math|Float|Max(Float) (- inputPercentage (/ (Math|Conversions|ToFloat(Integer) (+ _array_index 1)) (Math|Conversions|ToFloat(Integer) (Utilities|Array|Length _splinemeshes)))) 0.0) inputDelay) 1.0) inputPower) (Math|Float|Power (Math|Float|Min(Float) (/ (Math|Float|Max(Float) (- inputPercentage (/ (Math|Conversions|ToFloat(Integer) (+ _array_index 1)) (Math|Conversions|ToFloat(Integer) (Utilities|Array|Length _splinemeshes)))) 0.0) inputDelay) 1.0) inputPower))) true :!class /Script/Engine.SplineMeshComponent)))
    (:then_1
      ;[1 1 1] Static Meshes
      (LocalVariables|SetstaticMeshes_num_index 0)
      (LocalVariables|SetstaticMeshes_num_sum 0)
      (for (_array_element_2 _array_index_2) (Variables|Default|GetstaticMeshes)
        (if (>= _array_index_2 (+ (Utilities|Array|Get(acopy) (Variables|Default|GetstaticMeshes_num) (LocalVariables|GetstaticMeshes_num_index)) (LocalVariables|GetstaticMeshes_num_sum)))
          (LocalVariables|SetstaticMeshes_num_sum (+ (LocalVariables|GetstaticMeshes_num_sum) (Utilities|Array|Get(acopy) (Variables|Default|GetstaticMeshes_num) (LocalVariables|GetstaticMeshes_num_index))))
          (LocalVariables|SetstaticMeshes_num_index (+ (LocalVariables|GetstaticMeshes_num_index) 1)))
        (Transformation|SetRelativeScale3D _array_element_2 (Math|Vector|MakeVector (Math|Float|Lerp (.X (Math|Vector|BreakVector (Utilities|Array|Get(acopy) (Variables|Default|GetstaticMeshes_scale) _array_index_2))) (.X (Math|Vector|BreakVector (* (Utilities|Array|Get(acopy) (Variables|Default|GetstaticMeshes_scale) _array_index_2) (Math|Float|Power (Math|Float|Min(Float) (/ (Math|Float|Max(Float) (- inputPercentage (/ (Math|Conversions|ToFloat(Integer) (- _array_index_2 (LocalVariables|GetstaticMeshes_num_sum))) (Math|Conversions|ToFloat(Integer) (Utilities|Array|Get(acopy) (Variables|Default|GetstaticMeshes_num) (LocalVariables|GetstaticMeshes_num_index))))) 0.0) (Utilities|Array|Get(acopy) inputDelay_staticMesh (LocalVariables|GetstaticMeshes_num_index))) 1.0) (Utilities|Array|Get(acopy) inputPower_staticMesh (LocalVariables|GetstaticMeshes_num_index)))))) (.X (Class|KismetMathLibrary|BreakVector3f (Utilities|Array|Get(acopy) inputAxis_staticMesh (LocalVariables|GetstaticMeshes_num_index))))) (Math|Float|Lerp (.Y (Math|Vector|BreakVector (Utilities|Array|Get(acopy) (Variables|Default|GetstaticMeshes_scale) _array_index_2))) (.Y (Math|Vector|BreakVector (* (Utilities|Array|Get(acopy) (Variables|Default|GetstaticMeshes_scale) _array_index_2) (Math|Float|Power (Math|Float|Min(Float) (/ (Math|Float|Max(Float) (- inputPercentage (/ (Math|Conversions|ToFloat(Integer) (- _array_index_2 (LocalVariables|GetstaticMeshes_num_sum))) (Math|Conversions|ToFloat(Integer) (Utilities|Array|Get(acopy) (Variables|Default|GetstaticMeshes_num) (LocalVariables|GetstaticMeshes_num_index))))) 0.0) (Utilities|Array|Get(acopy) inputDelay_staticMesh (LocalVariables|GetstaticMeshes_num_index))) 1.0) (Utilities|Array|Get(acopy) inputPower_staticMesh (LocalVariables|GetstaticMeshes_num_index)))))) (.Y (Class|KismetMathLibrary|BreakVector3f (Utilities|Array|Get(acopy) inputAxis_staticMesh (LocalVariables|GetstaticMeshes_num_index))))) (Math|Float|Lerp (.Z (Math|Vector|BreakVector (Utilities|Array|Get(acopy) (Variables|Default|GetstaticMeshes_scale) _array_index_2))) (.Z (Math|Vector|BreakVector (* (Utilities|Array|Get(acopy) (Variables|Default|GetstaticMeshes_scale) _array_index_2) (Math|Float|Power (Math|Float|Min(Float) (/ (Math|Float|Max(Float) (- inputPercentage (/ (Math|Conversions|ToFloat(Integer) (- _array_index_2 (LocalVariables|GetstaticMeshes_num_sum))) (Math|Conversions|ToFloat(Integer) (Utilities|Array|Get(acopy) (Variables|Default|GetstaticMeshes_num) (LocalVariables|GetstaticMeshes_num_index))))) 0.0) (Utilities|Array|Get(acopy) inputDelay_staticMesh (LocalVariables|GetstaticMeshes_num_index))) 1.0) (Utilities|Array|Get(acopy) inputPower_staticMesh (LocalVariables|GetstaticMeshes_num_index)))))) (.Z (Class|KismetMathLibrary|BreakVector3f (Utilities|Array|Get(acopy) inputAxis_staticMesh (LocalVariables|GetstaticMeshes_num_index)))))))))))

(fn GrowUpbyPercentage
  (params (inputPercentage :type Float%20%28double-precision%29)))