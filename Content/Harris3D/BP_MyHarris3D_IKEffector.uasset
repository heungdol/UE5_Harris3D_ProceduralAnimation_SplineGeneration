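; Harris 3D effector actor that offers selected vertex locations and normals as IK targets for hands and feet.
; Its box overlap adds or removes it from the ThirdPersonCharacter's Harris list.
; GetClosestEffector picks the nearest point within distance limits that passes a normal-direction dot test and an occlusion trace from the pelvis; the vertex-type filter is unused.
; Helper getters return a point's location, normal, type, and per-limb rotations built from normal and forward vectors.
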(event OnComponentBeginOverlap(Box)
  (params (OverlappedComponent :type Primitive%20Component%20Object%20Reference) (OtherActor :type Actor%20Object%20Reference) (OtherComp :type Primitive%20Component%20Object%20Reference) (OtherBodyIndex :type Integer) (bFromSweep :type Boolean) (SweepResult :type Hit%20Result%20Structure%20%28by%20ref%29))
  (bind _asthird_person_character (Utilities|Casting|CastToThirdPersonCharacter OtherActor))
  (Default|AddHarristoList _asthird_person_character self))

(event OnComponentEndOverlap(Box)
  (params (OverlappedComponent :type Primitive%20Component%20Object%20Reference) (OtherActor :type Actor%20Object%20Reference) (OtherComp :type Primitive%20Component%20Object%20Reference) (OtherBodyIndex :type Integer))
  (bind _asthird_person_character (Utilities|Casting|CastToThirdPersonCharacter OtherActor))
  (Default|DeleteHarrisfromList _asthird_person_character self))

(event EventBeginPlay)

(event Collision|EventActorBeginOverlap
  (params (OtherActor :type Actor%20Object%20Reference)))

(event EventTick
  (params (DeltaSeconds :type Float%20%28single-precision%29)))

(fn ConstructionScript
  (bind _boxcolliderscale (Variables|Default|GetBoxColliderScale))
  (bind _box (Variables|Default|GetBox))
  (Components|Box|SetBoxExtent _box _boxcolliderscale true)
  (Transformation|SetRelativeLocation _box (Math|Vector|MakeVector 0.0 0.0 (.Z (Math|Vector|BreakVector _boxcolliderscale))) false false))

(fn GetClosestEffector
  (params (inputLoc :type Vector) (inputPelvis :type Vector) (inputLimit_Max :type Float%20%28double-precision%29) (inputLimit_Min :type Float%20%28double-precision%29) (inputConditionDir :type Vector) (inputConditionDot :type Float%20%28double-precision%29))
  ;[1 1 1] 유효성 판단
  (if (<= (Utilities|Array|Length (Variables|Default|GetcurrentVrtLocs_postSelected)) 0)
    (return -1)
    (else
      ;[1 1 1] 초기화
      (LocalVariables|SetminDist 1e+03)
      (LocalVariables|SetcurtIndex -1)
      (LocalVariables|SetretLoc "0, 0, 0")
      ;[1 1 1] 반복
      (for (_array_element _array_index) (Variables|Default|GetcurrentVrtLocs_postSelected)
        ;[1 1 1] 조건 - 노멀
        (bind (_nor _bo) (CallFunction|GetEffectorNorbyIndex _array_index))
        ;[1 1 1] 조건 - 버텍스 타입
        (bind _outputtype (CallFunction|GetEffectorTypebyIndex))
        (if true
          ;[1 1 1] 두개 이상의 Harris 정보를 가져올 때의 이상한 움직임의 방지를 위함 (미흡함)
          (bind (_outhit _returnvalue) (Collision|LineTraceByChannel inputPelvis _array_element "TraceTypeQuery1" true 0 "None"))
          (if _returnvalue
            (if (< (Math|Float|Absolute(Float) (- (Math|Vector|Distance(Vector) (.Location (Collision|BreakHitResult _outhit)) inputPelvis) (Math|Vector|Distance(Vector) _array_element inputPelvis))) 0.1)
              (if (Math|Boolean|ANDBoolean (< (Math|Vector|Distance(Vector) _array_element inputLoc) inputLimit_Max) (and (> (Math|Vector|DotProduct inputConditionDir _nor) inputConditionDot) _bo) (> (Math|Vector|Distance(Vector) _array_element inputLoc) inputLimit_Min)) :!label _label
                ;[1 1 1] 가장 처음으로 하나 선택했을 때
                (if (== (LocalVariables|GetcurtIndex) -1)
                  (LocalVariables|SetminDist (Math|Vector|Distance(Vector) inputLoc _array_element))
                  (LocalVariables|SetretLoc _array_element)
                  (LocalVariables|SetcurtIndex _array_index)
                  (else
                    ;[1 1 1] 미리 선택한 위치와 비교
                    (if (< (Math|Vector|Distance(Vector) inputLoc _array_element) (LocalVariables|GetminDist))
                      (LocalVariables|SetminDist (Math|Vector|Distance(Vector) inputLoc _array_element))
                      (LocalVariables|SetretLoc _array_element)
                      (LocalVariables|SetcurtIndex _array_index))))))
            (else
              (goto _label)))))
      ;[1 1 1] 마무리
      (return (LocalVariables|GetcurtIndex)))))

(fn GetEffectorLocbyIndex
  (params (ind :type Integer))
  (if (!= ind -1)
    (return (Utilities|Array|Get(acopy) (Variables|Default|GetcurrentVrtLocs_postSelected) ind) true)
    (else
      (return "0, 0, 0" false))))

(fn GetEffectorNorbyIndex
  (params (ind :type Integer))
  (if (!= ind -1)
    (return (Utilities|Array|Get(acopy) (Variables|Default|GetcurrentVrtNors_postSelected) ind) true)
    (else
      (return "0, 0, 0" false))))

(fn GetEffectorRotbyIndexHandLeft
  (params (ind :type Integer) (forward :type Vector))
  (bind (_nor _bo) (CallFunction|GetEffectorNorbyIndex ind))
  (if _bo
    (bind _output_get (LocalVariables|Setnormal _nor))
    (return (Class|KismetMathLibrary|MakeRotfromYX _output_get forward) true)
    (else
      (return "0, 0, 0" false))))

(fn GetEffectorRotbyIndexHandRight
  (params (ind :type Integer) (forward :type Vector))
  (bind (_nor _bo) (CallFunction|GetEffectorNorbyIndex ind))
  (if _bo
    (bind _output_get (LocalVariables|Setnormal _nor))
    (return (Class|KismetMathLibrary|MakeRotfromYX (* _output_get -1.0) (* forward -1.0)) true)
    (else
      (return "0, 0, 0" false))))

(fn GetEffectorRotbyIndexFootLeft
  (params (ind :type Integer) (forward :type Vector))
  (bind (_nor _bo) (CallFunction|GetEffectorNorbyIndex ind))
  (if _bo
    (bind _output_get (LocalVariables|Setnormal _nor))
    (return (Math|Rotator|MakeRotfromXY _output_get (* forward -1.0)) true)
    (else
      (return "0, 0, 0" false))))

(fn GetEffectorRotbyIndexFootRight
  (params (ind :type Integer) (forward :type Vector))
  (bind (_nor _bo) (CallFunction|GetEffectorNorbyIndex ind))
  (if _bo
    (bind _output_get (LocalVariables|Setnormal _nor))
    (return (Math|Rotator|MakeRotfromXY (* _output_get -1.0) (* forward 1.0)) true)
    (else
      (return "0, 0, 0" false))))

(fn GetEffectorTypebyIndex
  (params (inputIndex :type Integer))
  (if (!= inputIndex -1)
    (return (Utilities|Array|Get(acopy) (Variables|Default|GetvrtTypes_postSelected) inputIndex))
    (else
      (return "NONE"))))