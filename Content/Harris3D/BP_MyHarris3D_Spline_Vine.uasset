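; Harris3D spline Blueprint for a procedural vine with a stem and leaves that grow by percentage.
; It chains points greedily across Harris3D vertices, picking the nearest within a distance band that passes growth-direction and normal dot tests, and packs mesh and vertex indices into one buffer.
; Initialization builds a stem pipe and spaced leaf meshes along the spline.
; GrowUpByPercentage passes separate stem and leaf power and delay to GrowUpByInfos.
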(event EventBeginPlay
  (|CallParentFunction) ; This node is disabled and will not be called.\nDrag off pins to build functionality.
)

(event Collision|EventActorBeginOverlap
  (params (OtherActor :type Actor%20Object%20Reference))
  (|CallParentFunction OtherActor) ; This node is disabled and will not be called.\nDrag off pins to build functionality.
)

(event EventTick
  (params (DeltaSeconds :type Float%20%28single-precision%29))
  (|CallParentFunction DeltaSeconds) ; This node is disabled and will not be called.\nDrag off pins to build functionality.
)

(event EventInitializeHarris3DSpline
  (bind _spline (Variables|Default|GetSpline))
  (bind _outputsuccess (CallFunction|InitSplinePre))
  (if _outputsuccess
    (CallFunction|InitSpline)
    (CallFunction|InitSplineMeshPipe _spline (Variables|Default|Getstem_mesh) (Variables|Default|Getstem_mesh_axis) (Variables|Default|Getstem_mesh_scale) 1.0 0.0 (Variables|Default|Getstem_offset))
    (CallFunction|InitSplineMeshDistance _spline (Variables|Default|Getleaf_mesh) (Variables|Default|Getleaf_mesh_axis) (Variables|Default|Getleaf_mesh_scale) (Variables|Default|Getleaf_mesh_scale_random) 1.0 0.7 (Variables|Default|Getleaf_mesh_space) (Variables|Default|Getleaf_offset))))

(fn ConstructionScript)

(fn GetPointfromHarris3DVine
  (params (inputHarris3D :type My%20Harris%203D%20Object%20Reference) (inputLocation :type Vector) (inputDistMin :type Float%20%28double-precision%29) (inputDistMax :type Float%20%28double-precision%29) (inputDotXY :type Float%20%28double-precision%29) (inputDotZ :type Float%20%28double-precision%29) (inputUpVector :type Vector))
  (if (<= (Utilities|Array|Length (Variables|/Script/Harris3D.MyHarris3D|GetcurrentVrtLocs_postSelected inputHarris3D)) 0)
    (return -1)
    (else
      (LocalVariables|SetcurrentIndex -1)
      (LocalVariables|SetcurrentDist 1e+04)
      (LocalVariables|SetcurrentDir "0, 0,1.000000")
      (for _index (range 0 (- (Utilities|Array|Length (Variables|/Script/Harris3D.MyHarris3D|GetcurrentVrtLocs_postSelected inputHarris3D)) 1))
        ;[1 1 1] Upper
        (if true
          ;[1 1 1] Dist
          (if (and (> (Math|Vector|Distance(Vector) inputLocation (Utilities|Array|Get(acopy) (Variables|/Script/Harris3D.MyHarris3D|GetcurrentVrtLocs_postSelected inputHarris3D) _index)) inputDistMin) (< (Math|Vector|Distance(Vector) inputLocation (Utilities|Array|Get(acopy) (Variables|/Script/Harris3D.MyHarris3D|GetcurrentVrtLocs_postSelected inputHarris3D) _index)) inputDistMax))
            ;[1 1 1] Dot->Z
            (if (> (Math|Vector|DotProduct (Math|Vector|Normalize (- (Utilities|Array|Get(acopy) (Variables|/Script/Harris3D.MyHarris3D|GetcurrentVrtLocs_postSelected inputHarris3D) _index) inputLocation)) inputUpVector) (Math|Float|Clamp(Float) inputDotZ))
              ;[1 1 1] Dot->XY
              (if (> (Math|Vector|DotProduct (LocalVariables|GetcurrentDir) (Utilities|Array|Get(acopy) (Variables|/Script/Harris3D.MyHarris3D|GetcurrentVrtNors_postSelected inputHarris3D) _index)) inputDotXY)
                ;[1 1 1] Best
                (if (< (Math|Vector|Distance(Vector) inputLocation (Utilities|Array|Get(acopy) (Variables|/Script/Harris3D.MyHarris3D|GetcurrentVrtLocs_postSelected inputHarris3D) _index)) (LocalVariables|GetcurrentDist))
                  (LocalVariables|SetcurrentDist (Math|Vector|Distance(Vector) inputLocation (Utilities|Array|Get(acopy) (Variables|/Script/Harris3D.MyHarris3D|GetcurrentVrtLocs_postSelected inputHarris3D) _index)))
                  (LocalVariables|SetcurrentIndex _index)
                  (LocalVariables|SetcurrentDir (Utilities|Array|Get(acopy) (Variables|/Script/Harris3D.MyHarris3D|GetcurrentVrtNors_postSelected inputHarris3D) _index))))))))
      (return (LocalVariables|GetcurrentIndex)))))

(fn GetPointsfromHarris3D
  (params (inputStartPoints :type Vector :default "0, 0, 0"))
  (LocalVariables|SetloopLocation inputStartPoints)
  (LocalVariables|SetloopConditionTotal true)
  (bind _index (Utilities|FlowControl|ForLoopwithBreak 0 (- (Utilities|Array|Length (Variables|Default|GetmyHarris3Ds)) 1) :!label _label)
    (:LoopBody
      (if (LocalVariables|GetloopConditionTotal)
        (LocalVariables|SetloopCondition true)
        (while (LocalVariables|GetloopCondition)
          (bind _outputindex (CallFunction|GetPointfromHarris3DVine (Utilities|Array|Get(acopy) (Variables|Default|GetmyHarris3Ds) _index) (LocalVariables|GetloopLocation) (Variables|Default|Getspline_detect_dist_min) (Variables|Default|Getspline_detect_dist_max) 0.0 0.0 (Variables|Default|Getspline_detect_direction)))
          (if (== _outputindex -1)
            (LocalVariables|SetloopCondition false)
            (if (== _index (- (Utilities|Array|Length (Variables|Default|GetmyHarris3Ds)) 1))
              (LocalVariables|SetloopConditionTotal false))
            (else
              (LocalVariables|SetloopLocation (Utilities|Array|Get(acopy) (Variables|/Script/Harris3D.MyHarris3D|GetcurrentVrtLocs_postSelected (Utilities|Array|Get(acopy) (Variables|Default|GetmyHarris3Ds) _index)) _outputindex))
              (Utilities|Array|Add (Variables|Default|GetindexBufferArray) (+ _outputindex (* _index (Variables|Default|GetvertexNum_max)))))))
        (else
          (goto _label Break))))))

(fn GrowUpbyPercentage
  (params (inputPercentage :type Float%20%28double-precision%29))
  (bind _powers (LocalVariables|Getpowers))
  (bind _delays (LocalVariables|Getdelays))
  (Utilities|Array|Clear _powers)
  (Utilities|Array|Clear _delays)
  (Utilities|Array|Clear (LocalVariables|Getaxises))
  (Utilities|Array|Add _powers (Variables|Default|Getleaf_growth_power))
  (Utilities|Array|Add _delays (Variables|Default|Getleaf_growth_delay))
  (Utilities|Array|Add (LocalVariables|Getaxises) "1.000000,1.000000,1.000000")
  (CallFunction|GrowUpbyInfos inputPercentage (Variables|Default|Getstem_growth_power) (Variables|Default|Getstem_growth_delay) (LocalVariables|Getpowers) (LocalVariables|Getdelays) (LocalVariables|Getaxises)))