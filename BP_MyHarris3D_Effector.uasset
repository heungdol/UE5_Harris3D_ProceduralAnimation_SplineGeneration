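; BP_MyHarris3D_Effector offers preselected surface vertices as hand and foot effector targets for the ThirdPersonCharacter.
; Its box collider, sized at BeginPlay, adds or removes it from the character's list on overlap.
; GetClosestEffector picks the nearest vertex that passes a pelvis line-of-sight trace, range limit and normal-direction dot test, returning its index.
; Index lookups return location, normal and per-limb rotations built from normal and forward vector.
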(event OnComponentBeginOverlap(Box)
  (params (OverlappedComponent :type Primitive%20Component%20Object%20Reference) (OtherActor :type Actor%20Object%20Reference) (OtherComp :type Primitive%20Component%20Object%20Reference) (OtherBodyIndex :type Integer) (bFromSweep :type Boolean) (SweepResult :type Hit%20Result%20Structure%20%28by%20ref%29))
  (bind _asthird_person_character (Utilities|Casting|CastToThirdPersonCharacter OtherActor))
  (Default|AddHarristoList _asthird_person_character self))

(event OnComponentEndOverlap(Box)
  (params (OverlappedComponent :type Primitive%20Component%20Object%20Reference) (OtherActor :type Actor%20Object%20Reference) (OtherComp :type Primitive%20Component%20Object%20Reference) (OtherBodyIndex :type Integer))
  (bind _asthird_person_character (Utilities|Casting|CastToThirdPersonCharacter OtherActor))
  (Default|DeleteHarrisfromList _asthird_person_character self))

(event EventBeginPlay
  (bind _boxcolliderscale (Variables|Default|GetBoxColliderScale))
  (bind _box (Variables|Default|GetBox))
  (Components|Box|SetBoxExtent _box _boxcolliderscale true)
  (Transformation|SetRelativeLocation _box (Math|Vector|MakeVector 0.0 0.0 (.Z (Math|Vector|BreakVector _boxcolliderscale))) false false))

(event Collision|EventActorBeginOverlap
  (params (OtherActor :type Actor%20Object%20Reference)))

(event EventTick
  (params (DeltaSeconds :type Float%20%28single-precision%29)))

(fn ConstructionScript)

(fn GetClosestEffector
  (params (inputLoc :type Vector) (inputLoc_detect :type Vector) (inputPelvis :type Vector) (inputLimit :type Float%20%28double-precision%29) (inputConditionDir :type Vector) (inputConditionDot :type Float%20%28double-precision%29))
  ;[1 1 1] 길이 검사
  (if (<= (Utilities|Array|Length (Variables|Default|GetcurrentVrtLocs_postSelected)) 0)
    (return -1)
    (else
      ;[1 1 1] 초기 세팅
      (LocalVariables|SetminDist 1e+03)
      (LocalVariables|SetcurtIndex -1)
      (LocalVariables|SetretLoc "0, 0, 0")
      ;[1 1 1] 루프
      (for (_array_element _array_index) (Variables|Default|GetcurrentVrtLocs_postSelected)
        (bind (_nor _bo) (CallFunction|GetEffectorNorbyIndex _array_index))
        (bind (_outhit _returnvalue) (Collision|LineTraceByChannel inputPelvis _array_element "TraceTypeQuery1" true 0 "None"))
        (if _returnvalue
          (if (< (Math|Float|Absolute(Float) (- (Math|Vector|Distance(Vector) (.Location (Collision|BreakHitResult _outhit)) inputPelvis) (Math|Vector|Distance(Vector) _array_element inputPelvis))) 0.1)
            (if (and (< (Math|Vector|Distance(Vector) _array_element inputLoc_detect) inputLimit) (and (> (Math|Vector|DotProduct inputConditionDir _nor) inputConditionDot) _bo)) :!label _label
              (if (== (LocalVariables|GetcurtIndex) -1)
                (LocalVariables|SetminDist (Math|Vector|Distance(Vector) inputLoc _array_element))
                (LocalVariables|SetretLoc _array_element)
                (LocalVariables|SetcurtIndex _array_index)
                (elif (< (Math|Vector|Distance(Vector) inputLoc _array_element) (LocalVariables|GetminDist))
                  (LocalVariables|SetminDist (Math|Vector|Distance(Vector) inputLoc _array_element))
                  (LocalVariables|SetretLoc _array_element)
                  (LocalVariables|SetcurtIndex _array_index)))))
          (else
            (goto _label))))
      (return (LocalVariables|GetcurtIndex)))))

(fn GetEffectorLocbyIndex
  (params (ind :type Integer))
  (if (!= ind -1)
    (return (Utilities|Array|Get(acopy) (Variables|Default|GetcurrentVrtLocs_postSelected) ind) true)
    (else
      (return "0, 0, 0" false))))

(fn GetEffectorNorbyIndex
  (params (ind :type Integer))
  (if (!= ind -1)
    (return (Utilities|Array|Get(acopy) (Variables|Default|GetcurrentVrtNors_postSelected) ind) true)
    (else
      (return "0, 0, 0" false))))

(fn GetEffectorRotbyIndexHandLeft
  (params (ind :type Integer) (forward :type Vector))
  (bind (_nor _bo) (CallFunction|GetEffectorNorbyIndex ind))
  (if _bo
    (bind _output_get (LocalVariables|Setnormal _nor))
    (return (Class|KismetMathLibrary|MakeRotfromYX _output_get forward) true)
    (else
      (return "0, 0, 0" false))))

(fn GetEffectorRotbyIndexHandRight
  (params (ind :type Integer) (forward :type Vector))
  (bind (_nor _bo) (CallFunction|GetEffectorNorbyIndex ind))
  (if _bo
    (bind _output_get (LocalVariables|Setnormal _nor))
    (return (Class|KismetMathLibrary|MakeRotfromYX (* _output_get -1.0) (* forward -1.0)) true)
    (else
      (return "0, 0, 0" false))))

(fn GetEffectorRotbyIndexFootLeft
  (params (ind :type Integer) (forward :type Vector))
  (bind (_nor _bo) (CallFunction|GetEffectorNorbyIndex ind))
  (if _bo
    (bind _output_get (LocalVariables|Setnormal _nor))
    (return (Math|Rotator|MakeRotfromXY _output_get (* forward -1.0)) true)
    (else
      (return "0, 0, 0" false))))

(fn GetEffectorRotbyIndexFootRight
  (params (ind :type Integer) (forward :type Vector))
  (bind (_nor _bo) (CallFunction|GetEffectorNorbyIndex ind))
  (if _bo
    (bind _output_get (LocalVariables|Setnormal _nor))
    (return (Math|Rotator|MakeRotfromXY (* _output_get -1.0) (* forward 1.0)) true)
    (else
      (return "0, 0, 0" false))))